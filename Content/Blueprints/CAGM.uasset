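; CAGM is the game mode that manages saved settings, the main menu and a Socket.IO link for sending light updates.
; On BeginPlay it binds the "chat message" event, loads or creates the CALightSave, then shows the main menu with the mouse cursor.
; Connect uses the server address stored in the save.
; UpdateLights serializes its struct to JSON and emits it as a "chat message".
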(event `self.ReceiveBeginPlay`
  (`self.BindSocket`)
  (bind _returnvalue (`GameplayStatics.DoesSaveGameExist` (`self.SaveGameName`)))
  (if _returnvalue
    (bind _returnvalue_2 (`GameplayStatics.LoadGameFromSlot` (`self.SaveGameName`)))
    (set `self.SaveGameRef` _returnvalue_2)
    (else
      (bind _returnvalue_3 (`GameplayStatics.CreateSaveGameObject` "/Game/CALightSave.CALightSave_C"))
      (bind _output_get (set `self.SaveGameRef` _returnvalue_3))
      (`GameplayStatics.SaveGameToSlot` _output_get (`self.SaveGameName`))))
  (bind _returnvalue_4 (`|CreateWidget` "/Game/UI/MainMenu.MainMenu_C"))
  (`UserWidget.AddToViewport` _returnvalue_4 0)
  (set `PlayerController.bShowMouseCursor` true (`GameplayStatics.GetPlayerController` 0)))

(event `SaveGame`
  (`GameplayStatics.SaveGameToSlot` (`self.SaveGameRef`) (`self.SaveGameName`)))

(event `LoadGame`
  (`GameplayStatics.LoadGameFromSlot` (`self.SaveGameName`)))

(event `BindSocket`
  (`SocketIOClientComponent.BindEvent` (`self.SocketIOClient`) "chat message" "/"))

(event `socketConnect`
  (bind (_server_servername _server_serveraddress) (break `/Game/ServerStruct` (`/Game/CALightSave.Server` (cast `/Game/CALightSave` (`/Game/Blueprints/CAGM.SaveGameRef` (cast `/Game/Blueprints/CAGM` (`GameplayStatics.GetGameMode`) :!pure true)) :!pure true))))
  (`KismetSystemLibrary.PrintString` "connect to socket server")
  (`SocketIOClientComponent.Connect` (`self.SocketIOClient`) _server_serveraddress null null))

(event `socketDisconnect`
  (`KismetSystemLibrary.PrintString` "disconnect from socket server")
  (`SocketIOClientComponent.Disconnect` (`self.SocketIOClient`)))

(event `self.SocketIOClient.OnConnected`
  (params (SessionId :type String)))

(event `UpdateLights`
  (params (NewParam :type "/Game/LightStruct Structure"))
  (`SocketIOClientComponent.Emit` (`self.SocketIOClient`) "chat message" (`SIOJLibrary.Conv_JsonObjectToJsonValue` (`SIOJLibrary.StructToJsonObject` NewParam)) "/"))

(fn `UserConstructionScript`)